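; HouseDoor_BP is an interactable house door that swings its static mesh open and closed.
; The Interactwith event checks the mesh's relative yaw, reversing the DoorAnimation timeline if the door is near fully open and playing it otherwise.
; The timeline's Update handler lerps yaw between closed and a quarter turn using its Alpha track, so the rotation itself serves as the open state.
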(event EventInteractwith
  (bind _dooranimation (Variables|Default|GetDoorAnimation))
  (if (Math|Float|NearlyEqual(Float) (.yaw (Variables|/Script/Engine.SceneComponent|GetRelativeRotation (Variables|Default|GetStaticMesh))) -9e+01 5.0)
    (Utilities|String|Reverse _dooranimation)
    (else
      (Audio|Components|Audio|Play _dooranimation))))

(fn ConstructionScript)